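; FBos is a boss enemy that uses PawnSensing to attack the ThirdPersonCharacter.
; On seeing the player, it turns to face them and spawns BossShotTwo at ProjectileSpawnLocation.
; SpawnFire resets on every sighting, so its 0.1-second delay never limits the fire rate.
; Tick and heard noise both subtract slight FullHealth from the cast Pawn, while movement, lava floor and impulse logic are unconnected.
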(event OnSeePawn(PawnSensing)
  (params (Pawn :type Pawn%20Object%20Reference))
  (bind _asthird_person_character (Utilities|Casting|CastToThirdPersonCharacter Pawn))
  (Utilities|FlowControl|Sequence
    (:then_0
      (Transformation|SetActorRotation (Math|Rotator|FindLookatRotation (Transformation|GetActorLocation) (Transformation|GetActorLocation _asthird_person_character)))
      (Variables|Default|SetSpawnFire true))
    (:then_1
      (if (Variables|Default|GetSpawnFire)
        (Game|SpawnActorfromClass "/Game/Blueprints/Interactables/projectiles/BossShotTwo.BossShotTwo_C" (Transformation|GetWorldTransform (Variables|Default|GetProjectileSpawnLocation)) "Undefined" 0 0)
        (Variables|Default|SetSpawnFire false)
        (Utilities|FlowControl|Delay 0.1)
        (Variables|Default|SetSpawnFire true)))))

(event OnHearNoise(PawnSensing)
  (params (Instigator :type Pawn%20Object%20Reference) (Location :type Vector%20%28by%20ref%29 :default "0, 0, 0") (Volume :type Float%20%28single-precision%29))
  (bind _asthird_person_character (Utilities|Casting|CastToThirdPersonCharacter (stale OnSeePawn(PawnSensing) Pawn)))
  (Variables|/Game/ThirdPersonBP/Blueprints/ThirdPersonCharacter.ThirdPersonCharacter_C|SetFull%20Health _asthird_person_character (- (Variables|/Game/ThirdPersonBP/Blueprints/ThirdPersonCharacter.ThirdPersonCharacter_C|GetFull%20Health _asthird_person_character) 0.01)))

(event EventBeginPlay)

(event Collision|EventActorBeginOverlap
  (params (OtherActor :type Actor%20Object%20Reference)))

(event EventTick
  (params (DeltaSeconds :type Float%20%28single-precision%29))
  (bind _asthird_person_character (Utilities|Casting|CastToThirdPersonCharacter (stale OnSeePawn(PawnSensing) Pawn)))
  (Variables|/Game/ThirdPersonBP/Blueprints/ThirdPersonCharacter.ThirdPersonCharacter_C|SetFull%20Health _asthird_person_character (- (Variables|/Game/ThirdPersonBP/Blueprints/ThirdPersonCharacter.ThirdPersonCharacter_C|GetFull%20Health _asthird_person_character) 0.01)))

(fn ConstructionScript)