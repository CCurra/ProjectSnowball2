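; DamageSphere_Blueprint2 is a pickup-style trigger that drops the BarrierP2 actor when the first player's pawn touches its box.
; On overlap it destroys itself, then hides the barrier and disables its collision.
; The barrier's restore sits behind a three-second Delay on the already destroyed actor, so it likely never runs.
; Disconnected nodes would destroy the barrier and subtract health from an Iceboss.
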(event OnComponentBeginOverlap(Box)
  (params (OverlappedComponent :type Primitive%20Component%20Object%20Reference) (OtherActor :type Actor%20Object%20Reference) (OtherComp :type Primitive%20Component%20Object%20Reference) (OtherBodyIndex :type Integer) (bFromSweep :type Boolean) (SweepResult :type Hit%20Result%20Structure%20%28by%20ref%29))
  (bind _barrierp2 (Variables|Default|GetBarrierP2))
  (if (== OtherActor (Game|Player|GetPlayerPawn 0))
    (Actor|DestroyActor)
    (Collision|SetActorEnableCollision _barrierp2 false)
    (Rendering|SetActorHiddenInGame _barrierp2 true)
    (Utilities|FlowControl|Delay 3.0)
    (Development|PrintString "Hello")
    (Collision|SetActorEnableCollision _barrierp2 true)
    (Rendering|SetActorHiddenInGame _barrierp2 false)))

(event EventBeginPlay)

(event Collision|EventActorBeginOverlap
  (params (OtherActor :type Actor%20Object%20Reference)))

(event EventTick
  (params (DeltaSeconds :type Float%20%28single-precision%29)))

(fn ConstructionScript)