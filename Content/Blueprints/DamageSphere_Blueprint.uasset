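; DamageSphere is a trigger actor that destroys itself on overlap and disables the collision and visibility of a referenced BarrierP.
; Any actor overlap runs this sequence, as does the Box overlap when the player pawn enters.
; A three-second Delay should restore the barrier, but it follows the self-destruct, so it likely never completes.
; Logic subtracting Iceboss HP and destroying the barrier is left unconnected.
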(event OnComponentBeginOverlap(Box)
  (params (OverlappedComponent :type Primitive%20Component%20Object%20Reference) (OtherActor :type Actor%20Object%20Reference) (OtherComp :type Primitive%20Component%20Object%20Reference) (OtherBodyIndex :type Integer) (bFromSweep :type Boolean) (SweepResult :type Hit%20Result%20Structure%20%28by%20ref%29))
  (bind _barrierp (Variables|Default|GetBarrierP))
  (if (== OtherActor (Game|Player|GetPlayerPawn 0))
    (Actor|DestroyActor)
    (Collision|SetActorEnableCollision _barrierp false)
    (Rendering|SetActorHiddenInGame _barrierp true)
    (Utilities|FlowControl|Delay 3.0)
    (Development|PrintString "Hello")
    (Collision|SetActorEnableCollision _barrierp true)
    (Rendering|SetActorHiddenInGame _barrierp false)))

(event EventBeginPlay)

(event Collision|EventActorBeginOverlap
  (params (OtherActor :type Actor%20Object%20Reference))
  (bind _barrierp (Variables|Default|GetBarrierP))
  (Actor|DestroyActor)
  (Collision|SetActorEnableCollision _barrierp false)
  (Rendering|SetActorHiddenInGame _barrierp true)
  (Utilities|FlowControl|Delay 3.0)
  (Development|PrintString "Hello")
  (Collision|SetActorEnableCollision _barrierp true)
  (Rendering|SetActorHiddenInGame _barrierp false))

(event EventTick
  (params (DeltaSeconds :type Float%20%28single-precision%29)))

(fn ConstructionScript)