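; Puzzle box mover that repositions box actors when any actor overlaps it.
; Overlap plays a timeline from the start, whose updates set the root relative location of boxes one to four from per-box location values, without sweep.
; Unconnected work-in-progress logic would move boxes five to ten, disable cube collision and bind a second overlap handler that stores the player.
; The empty construction script and macro add nothing.
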(event Custom|OnActorBeginOverlap_Event_0
  (params (OverlappedActor :type Actor%20Object%20Reference) (OtherActor :type Actor%20Object%20Reference))
  ;[1 1 1] Refinement
  (Variables|Default|SetPlayer OverlappedActor))

(event Collision|EventActorBeginOverlap
  (params (OtherActor :type Actor%20Object%20Reference))
  ;[1 1 1] BoxMovementWorkinbg
  (Components|Timeline|PlayfromStart (Variables|Default|GetTimeLineBox1))
  (Development|PrintString "Hello")
  (Timeline|TimeLineBox1 Play
    (:Update
      (Transformation|SetRelativeLocation (Variables|/Script/Engine.Actor|GetRootComponent (Variables|Default|GetBoxOnePuzzle)) (Variables|Default|GetLocationSetOne) false false)
      (Transformation|SetRelativeLocation (Variables|/Script/Engine.Actor|GetRootComponent (Variables|Default|GetBoxTwoPuzzle)) (Variables|Default|GetLocationSetOneTwo) false false)
      (Transformation|SetRelativeLocation (Variables|/Script/Engine.Actor|GetRootComponent (Variables|Default|GetBoxThreePuzzle)) (Variables|Default|GetLocationSetThree) false false)
      (Transformation|SetRelativeLocation (Variables|/Script/Engine.Actor|GetRootComponent (Variables|Default|GetBoxFourPuzzle)) (Variables|Default|GetLocationSetFour) false false))))

(fn ConstructionScript)