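; Trigger button that rotates a platform when the player overlaps its box, presumably by 90 degrees given its name.
; On BeginPlay it stores the first Platform1 actor found in the level.
; The overlap plays a timeline that adds a fixed, swept local rotation to the platform's mesh each update, so the total depends on frame rate.
; A Start flag blocks retriggering until the timeline finishes.
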(event OnComponentBeginOverlap(Box)
  (params (OverlappedComponent :type Primitive%20Component%20Object%20Reference) (OtherActor :type Actor%20Object%20Reference) (OtherComp :type Primitive%20Component%20Object%20Reference) (OtherBodyIndex :type Integer) (bFromSweep :type Boolean) (SweepResult :type Hit%20Result%20Structure%20%28by%20ref%29))
  (if (== OtherActor (Game|Player|GetPlayerPawn 0))
    (if (not (Variables|Default|GetStart))
      (Variables|Default|SetStart true)
      (bind _asplatform_1 (Utilities|Casting|CastToplatform1 (Variables|Default|GetPlatform90)))
      (Timeline|Timeline_0 PlayFromStart
        (:Update
          (Transformation|AddLocalRotation (Variables|/Script/Engine.StaticMeshActor|GetStaticMeshComponent _asplatform_1) "0,0.500000,0.000000" true false))
        (:Finished
          (Variables|Default|SetStart false))))))

(event EventBeginPlay
  (bind _outactors (Actor|GetAllActorsOfClass "/Game/Blueprints/Interactables/rotatingPlatforms/platform1.platform1_C"))
  (Variables|Default|SetPlatform90 (Utilities|Array|Get(acopy) _outactors)))

(event Collision|EventActorBeginOverlap
  (params (OtherActor :type Actor%20Object%20Reference)))

(fn ConstructionScript)