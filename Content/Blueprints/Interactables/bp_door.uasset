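; Sliding double door actor that opens when the player pawn enters its Box trigger.
; The DoorTranstion timeline lerps Doorleft and DoorRight along relative Y in mirrored directions, with its play rate derived from DoorOpenTime.
; Ending an overlap reverses the timeline to close the door; unlike opening, this does not check that the actor is the player.
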(event OnComponentBeginOverlap(Box)
  (params (OverlappedComponent :type Primitive%20Component%20Object%20Reference) (OtherActor :type Actor%20Object%20Reference) (OtherComp :type Primitive%20Component%20Object%20Reference) (OtherBodyIndex :type Integer) (bFromSweep :type Boolean) (SweepResult :type Hit%20Result%20Structure%20%28by%20ref%29))
  (if (== (Game|Player|GetPlayerPawn 0) OtherActor)
    (Components|Timeline|SetPlayRate (Variables|Default|Getdoor%20transtion) (/ 1.0 (Variables|Default|Getdoor%20open%20time)))
    (bind _alpha (Timeline|door%20transtion Play)
      (:Update
        (Transformation|SetRelativeLocation (Variables|Default|Getdoorleft) (Math|Vector|MakeVector 0.0 (Math|Float|Lerp 1.1e+02 3.5e+02 _alpha) 0.0) false false)
        (Transformation|SetRelativeLocation (Variables|Default|Getdoor%20right%20) (Math|Vector|MakeVector 0.0 (* (Math|Float|Lerp 1.1e+02 3.5e+02 _alpha) -1.0) 0.0) false false)))))

(event OnComponentEndOverlap(Box)
  (params (OverlappedComponent :type Primitive%20Component%20Object%20Reference) (OtherActor :type Actor%20Object%20Reference) (OtherComp :type Primitive%20Component%20Object%20Reference) (OtherBodyIndex :type Integer))
  (Components|Timeline|SetPlayRate (Variables|Default|Getdoor%20transtion) (/ 1.0 (Variables|Default|Getdoor%20open%20time)))
  (bind _alpha (Timeline|door%20transtion Reverse)
    (:Update
      (Transformation|SetRelativeLocation (Variables|Default|Getdoorleft) (Math|Vector|MakeVector 0.0 (Math|Float|Lerp 1.1e+02 3.5e+02 _alpha) 0.0) false false)
      (Transformation|SetRelativeLocation (Variables|Default|Getdoor%20right%20) (Math|Vector|MakeVector 0.0 (* (Math|Float|Lerp 1.1e+02 3.5e+02 _alpha) -1.0) 0.0) false false))))

(event EventBeginPlay)

(event Collision|EventActorBeginOverlap
  (params (OtherActor :type Actor%20Object%20Reference)))

(event EventTick
  (params (DeltaSeconds :type Float%20%28single-precision%29)))

(fn ConstructionScript)