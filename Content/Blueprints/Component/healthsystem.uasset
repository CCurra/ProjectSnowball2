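; Health component that tracks an actor's current health and signals its death.
; Health starts at the maximum on BeginPlay, and a takedamage event subtracts incoming damage, printing a debug string on each non-lethal hit.
; Damage that meets or exceeds the remaining health passes through a DoOnce, which zeroes health and calls the death dispatcher a single time.
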(event Custom|take%20damage
  (params (damage :type Float%20%28single-precision%29))
  (if (>= damage (Variables|Default|Getcurrent%20health%20))
    (Utilities|FlowControl|DoOnce false
      (:Completed
        (Variables|Default|Setcurrent%20health%20 0.0)
        (Default|CallDeathDispacher)))
    (else
      (Variables|Default|Setcurrent%20health%20 (- (Variables|Default|Getcurrent%20health%20) damage))
      (Development|PrintString "outch"))))

(event EventBeginPlay
  (Variables|Default|Setcurrent%20health%20 (Variables|Default|Getmax%20health)))